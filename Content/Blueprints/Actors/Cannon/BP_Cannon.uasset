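; BP_Cannon is a cannon actor that automatically fires BP_Projectile instances in an endless loop from BeginPlay.
; After a FireRate delay, it spawns a scaled projectile at the ProjectileSpawnPoint's world location and rotation.
; The FireAnimation timeline then moves the barrel along its relative Y axis, and its Cannon Fired event loops back to the delay for the next shot.
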(event `self.ReceiveBeginPlay`
  (bind _projectilespawnpoint (`self.ProjectileSpawnPoint`))
  (`KismetSystemLibrary.Delay` (`self.FireRate`) :!label _label)
  (`|SpawnActorFromClass` "/Game/Blueprints/Actors/Projectiles/BP_Projectile.BP_Projectile_C" (`KismetMathLibrary.MakeTransform` (`SceneComponent.K2_GetComponentLocation` _projectilespawnpoint) (`SceneComponent.K2_GetComponentRotation` _projectilespawnpoint) (`KismetMathLibrary.Conv_DoubleToVector` (`self.ProjectileScale`))) "Undefined" "OverrideRootScale" null null)
  (bind (_direction _cannonbarrelmovement) (`Timeline|FireAnimation` :!via `PlayFromStart`)
    (:`Update`
      (`SceneComponent.K2_SetRelativeLocation` (`self.Cannon`) (`KismetMathLibrary.MakeVector` 0.0 _cannonbarrelmovement) false false))
    (:`CannonFired`
      (goto _label))))

(fn `UserConstructionScript`)