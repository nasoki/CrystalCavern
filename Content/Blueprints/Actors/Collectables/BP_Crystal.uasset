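; BP_Crystal is a collectable crystal that gets drawn into the player and vanishes when the player pawn overlaps it.
; On overlap it stores its location, scale and light intensity, then plays a timeline.
; The timeline's smoothed alpha lerps the actor toward the player's current position while shrinking it and fading its point light to zero.
; The actor destroys itself when the timeline finishes; no reward is granted here.
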(event `self.ReceiveActorBeginOverlap`
  (params (OtherActor :type "Actor Object Reference"))
  (`self.IsPlayer` OtherActor
    (:`IsPlayer`
      (`self.StoreStartingValues`)
      (bind (_direction _smoothlerpalpha) (`Timeline|AlphaBlendTimeline`)
        (:`Update`
          (`self.MoveToPlayer` _smoothlerpalpha)
          (`self.ScaleCrystals` _smoothlerpalpha)
          (`LightComponent.SetIntensity` (`self.PointLight`) (`KismetMathLibrary.Lerp` (`self.StartLightIntensity`) 0.0 _smoothlerpalpha)))
        (:`Finished`
          (`self.K2_DestroyActor`))))))

(fn `MoveToPlayer`
  (params (Alpha :type "Float (double-precision)"))
  (`self.K2_SetActorLocation` (`KismetMathLibrary.VLerp` (`self.LerpStartLocation`) (`self.K2_GetActorLocation` (`GameplayStatics.GetPlayerPawn` 0)) Alpha)))

(fn `ScaleCrystals`
  (params (Alpha :type "Float (double-precision)"))
  (`self.SetActorScale3D` (`KismetMathLibrary.VLerp` (`self.StartScale`) (0.0 0.0 0.0) Alpha)))

(fn `StoreStartingValues`
  (set `self.LerpStartLocation` (`self.K2_GetActorLocation`))
  (set `self.StartScale` (`self.GetActorScale3D`))
  (set `self.StartLightIntensity` (`LightComponentBase.Intensity` (`self.PointLight`))))

(fn `UserConstructionScript`)