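; BP_WinVolume is a level trigger that completes the current level when the player overlaps it and no BP_Crystal actors remain in the world.
; The crystal check uses GetAllActorsOfClass on each player overlap.
; On completion, it finds the current level in the ordered LevelNames array and opens the following entry by name.
; On the final level in that array, completion does nothing further.
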(event `self.ReceiveActorBeginOverlap`
  (params (OtherActor :type "Actor Object Reference"))
  (`/Game/Blueprints/Libraries/CC_MacroLibrary.IsPlayer` OtherActor
    (:`IsPlayer`
      (if (not (`self.AnyCrystalRemaining`))
        (`self.CompleteLevel`)))))

(fn `AnyCrystalRemaining`
  (returns (NewParam :type Boolean))
  (bind _outactors (`GameplayStatics.GetAllActorsOfClass` "/Game/Blueprints/Actors/Collectables/BP_Crystal.BP_Crystal_C"))
  (return (> (`KismetArrayLibrary.Array_Length` _outactors) 0)))

(fn `CompleteLevel`
  (if (not (`self.IsFinalLevel`))
    (`self.LoadNextLevel`)))

(fn `GetCurrentLevelIndex`
  (returns (ReturnValue :type Integer))
  (bind _returnvalue (`GameplayStatics.GetCurrentLevelName` true))
  (return (`KismetArrayLibrary.Array_Find` (`self.LevelNames`) (`KismetStringLibrary.Conv_StringToName` _returnvalue))))

(fn `GetNextLevelName`
  (returns (ReturnValue :type Name))
  (return (`|GetArrayItem` (`self.LevelNames`) (+ (`self.GetCurrentLevelIndex`) 1))))

(fn `IsFinalLevel`
  (returns (`Return Value` :type Boolean))
  (return (== (`KismetArrayLibrary.Array_LastIndex` (`self.LevelNames`)) (`self.GetCurrentLevelIndex`))))

(fn `LoadNextLevel`
  (`GameplayStatics.OpenLevel` (`self.GetNextLevelName`)))

(fn `UserConstructionScript`)